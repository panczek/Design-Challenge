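; BP_NoTeleportationZone is an interaction-based level object that disables VR teleportation for a motion controller pawn while the interaction lasts.
; It overrides its parent's InteractionTriggered to cast the interacting object's owner to MotionControllerPawn, cache it and clear AllowTeleport.
; InteractionEnd restores AllowTeleport on that cached pawn and clears the reference.
; The EventGraph holds only disabled events and unreachable copies of similar logic.
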(event EventBeginPlay)

(event Collision|EventActorBeginOverlap
  (params (OtherActor :type Actor%20Object%20Reference)))

(event EventTick
  (params (DeltaSeconds :type Float%20%28single-precision%29)))

(fn ConstructionScript)

(fn InteractionTriggered
  (|CallParentFunction)
  (bind _asmotion_controller_pawn (Utilities|Casting|CastToMotionControllerPawn (Components|GetOwner (Variables|Default|GetInteractObject))))
  (bind _output_get (Variables|Default|SetPawn _asmotion_controller_pawn))
  (Variables|/Game/DefaultVRContent/VirtualRealityBP/Blueprints/MotionControllerPawn.MotionControllerPawn_C|SetAllowTeleport _output_get false))

(fn InteractionEnd
  (|CallParentFunction)
  (Utilities|IsValid (Variables|Default|GetPawn)
    (:Is%20Valid
      (Variables|/Game/DefaultVRContent/VirtualRealityBP/Blueprints/MotionControllerPawn.MotionControllerPawn_C|SetAllowTeleport (Variables|Default|GetPawn) true))
    (:Is%20Not%20Valid
      _))
  (Variables|Default|SetPawn 0))