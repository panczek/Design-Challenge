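; BP_WebButton is an interactable level button that switches on a linked screen object when triggered.
; InteractionTriggered calls the parent logic, then, if the ScreenObject is valid, sets it activated and plays the button animation.
; The animation records the button's world position and uses a timeline Height value to offset it along its up vector.
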(event Custom|PlayAnimation
  (bind _button (Variables|Default|GetButton))
  (Variables|Default|SetStartPos (Transformation|GetWorldLocation _button))
  (bind _height (Timeline|Timeline PlayFromStart)
    (:Update
      (Transformation|SetWorldLocation (Variables|Default|GetButton) (+ (* _height (Math|Vector|GetUpVector _button)) (Variables|Default|GetStartPos)) false false))))

(fn ConstructionScript
  (|CallParentFunction))

(fn InteractionTriggered
  (bind _screenobject (Variables|Default|GetScreenObject))
  (|CallParentFunction)
  (Utilities|IsValid _screenobject
    (:Is%20Valid
      (Default|SetScreenActivated _screenobject true)
      (CallFunction|PlayAnimation))))