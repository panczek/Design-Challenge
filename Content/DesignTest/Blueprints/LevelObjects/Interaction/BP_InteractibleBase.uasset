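; Base interactible actor that responds when a BP_MotionController overlaps its Collision component.
; An optional direction check uses a dot product to accept only controllers on the side opposite the collision's up vector, and TriggerOnlyOnce blocks repeat triggers.
; Accepted overlaps store the controller and call InteractionTriggered, which sets IsTriggered.
; When that controller leaves, it updates CanActivate, calls the empty InteractionEnd hook and clears the reference.
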(event OnComponentBeginOverlap(Collision)
  (params (OverlappedComponent :type Primitive%20Component%20Object%20Reference) (OtherActor :type Actor%20Object%20Reference) (OtherComp :type Primitive%20Component%20Object%20Reference) (OtherBodyIndex :type Integer) (bFromSweep :type Boolean) (SweepResult :type Hit%20Result%20Structure%20%28by%20ref%29))
  (if (not (and (Variables|Setup|GetTriggerOnlyOnce) (Variables|Default|GetIsTriggered)))
    (bind _asbp_motion_controller (Utilities|Casting|CastToBP_MotionController OtherActor))
    (if (Variables|Setup|GetCheckDirection)
      (if (CallFunction|CheckInteractionDIrection (Transformation|GetActorLocation _asbp_motion_controller))
        (Variables|Default|SetInteractObject _asbp_motion_controller :!label _label)
        (CallFunction|InteractionTriggered))
      (else
        (goto _label)))))

(event OnComponentEndOverlap(Collision)
  (params (OverlappedComponent :type Primitive%20Component%20Object%20Reference) (OtherActor :type Actor%20Object%20Reference) (OtherComp :type Primitive%20Component%20Object%20Reference) (OtherBodyIndex :type Integer))
  (if (== OtherActor (Variables|Default|GetInteractObject))
    (Variables|Default|SetCanActivate (not (Variables|Setup|GetTriggerOnlyOnce)))
    (CallFunction|InteractionEnd)
    (Variables|Default|SetInteractObject 0)))

(event EventBeginPlay)

(event Collision|EventActorBeginOverlap
  (params (OtherActor :type Actor%20Object%20Reference)))

(event EventTick
  (params (DeltaSeconds :type Float%20%28single-precision%29)))

(fn ConstructionScript)

(fn CheckInteractionDIrection
  (params (Other%20Location :type Vector))
  (bind _collision (Variables|Default|GetCollision))
  (return (> (Math|Vector|DotProduct (Math|Vector|GetUpVector _collision) (Math|Vector|Normalize (- (Transformation|GetWorldLocation _collision) Other%20Location))) 0.0)))

(fn InteractionTriggered
  (Variables|Default|SetIsTriggered true))

(fn InteractionEnd)