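; BP_GrapplingSpline is a level object in DesignTest that lays out grapple points along a spline mesh.
; GeneratePointsAlongSpline destroys previous points, then spawns attached BP_GrapplingCube actors at fixed spacing on a straight line between the mesh's endpoints, ignoring curvature.
; A dot product detects overshoot, and a distance check triggers an extra cube at the end.
; The construction script is empty, Drop does nothing and Pickup only prints a debug string.
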(event EventBeginPlay)

(event Collision|EventActorBeginOverlap
  (params (OtherActor :type Actor%20Object%20Reference)))

(event EventTick
  (params (DeltaSeconds :type Float%20%28single-precision%29)))

(event EventDrop)

(event EventPickup
  (params (AttachTo :type Scene%20Component%20Object%20Reference) (Pawn :type Pawn%20Object%20Reference))
  (Development|PrintString "picked up"))

(fn ConstructionScript)

(fn GeneratePointsAlongSpline
  (bind _splinemeshcomponent (Variables|SplineMeshActor|GetSplineMeshComponent))
  (bind _splinemeshcomponent_2 (Variables|SplineMeshActor|GetSplineMeshComponent))
  (bind _returnvalue (SplineMesh|GetStartPosition _splinemeshcomponent))
  (bind _returnvalue_2 (SplineMesh|GetEndPosition _splinemeshcomponent))
  (bind _returnvalue_3 (SplineMesh|GetEndPosition _splinemeshcomponent_2))
  (bind _returnvalue_4 (- _returnvalue_2 _returnvalue))
  (for _array_element (Variables|Default|GetGraplingPoints)
    (Actor|DestroyActor _array_element))
  (LocalVariables|SetPointDelta (* (Variables|Default|GetDistanceBetweenPoints) (Math|Vector|Normalize _returnvalue_4)))
  (LocalVariables|SetPointLocation _returnvalue)
  (while (> (Math|Vector|DotProduct (- (SplineMesh|GetEndPosition (Variables|SplineMeshActor|GetSplineMeshComponent)) (LocalVariables|GetPointLocation)) _returnvalue_4) 0.0)
    (bind _returnvalue_5 (Game|SpawnActorfromClass "/Game/DesignTest/Blueprints/LevelObjects/BP_GrapplingCube.BP_GrapplingCube_C" (Math|Transform|MakeTransform (LocalVariables|GetPointLocation) "0, 0, 0" "1.000000,1.000000,1.000000") "Undefined" "MultiplyWithRoot" 0 0))
    (Transformation|AttachActorToActor _returnvalue_5 self "None" "KeepRelative" "KeepRelative" "KeepRelative" true)
    (Utilities|Array|AddUnique (Variables|Default|GetGraplingPoints) _returnvalue_5)
    (LocalVariables|SetPointLocation (+ (LocalVariables|GetPointLocation) (LocalVariables|GetPointDelta))))
  (if (> (Math|Vector|Distance(Vector) (LocalVariables|GetPointLocation) _returnvalue_3) (* (Variables|Default|GetDistanceBetweenPoints) 0.5))
    (LocalVariables|SetPointLocation _returnvalue_3)
    (bind _returnvalue_6 (Game|SpawnActorfromClass "/Game/DesignTest/Blueprints/LevelObjects/BP_GrapplingCube.BP_GrapplingCube_C" (Math|Transform|MakeTransform (LocalVariables|GetPointLocation) "0, 0, 0" "1.000000,1.000000,1.000000") "Undefined" "MultiplyWithRoot" 0 0))
    (Transformation|AttachActorToActor _returnvalue_6 self "None" "KeepRelative" "KeepRelative" "KeepRelative" true)
    (Utilities|Array|AddUnique (Variables|Default|GetGraplingPoints) _returnvalue_6)
    (LocalVariables|SetPointLocation (+ (LocalVariables|GetPointLocation) (LocalVariables|GetPointDelta)))))